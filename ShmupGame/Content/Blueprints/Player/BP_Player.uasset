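; Player pawn for a scrolling shooter that flies in with a spinning timeline animation before movement and firing unlock.
; Tick applies input-eased horizontal and vertical speeds, clamped to screen by BP_GameMode, and pitches the mesh with vertical speed.
; Looping timers fire primary and twin secondary projectiles, attached to the parallax camera.
; Collisions deflect movement; damage shakes the camera, and zero health triggers explosion, game over and destruction.
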(event `self.ReceiveBeginPlay`
  (bind _spawnlocation (`self.SpawnLocation`))
  ;[1 1 1] Player Spawn Animation
  (bind _asbp_game_mode (cast `/Game/Blueprints/BP_GameMode` (`GameplayStatics.GetGameMode`)))
  (set `self.BP_GameMode` _asbp_game_mode)
  (set `self.Pitch` (.pitch (`self.K2_GetActorRotation`)))
  (bind (_direction _speed) (`Timeline|SpawnAnimation`)
    (:`Update`
      (`self.K2_SetActorRelativeLocation` (`KismetMathLibrary.VLerp` _spawnlocation (+ _spawnlocation (0.0 1000.0 0.0)) _speed))
      (`self.K2_SetActorRelativeRotation` (`KismetMathLibrary.RLerp` (struct) (`KismetMathLibrary.MakeRotator` (+ (`self.Pitch`) (`self.SpawnSpinCount`)) 0.0 90.0) _speed)))
    (:`Finished`
      (set `self.MoveEnabled` true))))

(event `self.ReceiveTick`
  (params (DeltaSeconds :type "Float (single-precision)"))
  (bind _skeletalmesh (`self.SkeletalMesh`))
  ;[1 1 1] Player Movement
  (if (`self.MoveEnabled`)
    (set `self.DeltaSeconds` DeltaSeconds)
    (bind _outvec (`/Game/Blueprints/BP_GameMode.ClampToScreen` (`self.BP_GameMode`) (+ (`self.K2_GetActorLocation`) (`KismetMathLibrary.MakeVector` (`self.HSpeed`) 0.0 (`self.VSpeed`)))))
    (`self.K2_SetActorLocation` _outvec true)
    (`/Engine/EditorBlueprintResources/StandardMacros.IsValid` self
      (:`Is Valid`
        (`SceneComponent.K2_SetRelativeRotation` _skeletalmesh (`KismetMathLibrary.RInterpTo_Constant` (`SceneComponent.RelativeRotation` _skeletalmesh) (`KismetMathLibrary.MakeRotator` 0.0 (+ (* (`self.VSpeed`) -2.0) (`self.Pitch`)) -90.0) (`self.DeltaSeconds`) 80.0) false false)))))

(event `InputAxis|MoveUp`
  (params (AxisValue :type "Float (single-precision)"))
  ;[1 1 1] Player Input
  (bind _return_direction_speed (`self.Movement` AxisValue (`self.VSpeed`)))
  (set `self.VSpeed` _return_direction_speed))

(event `InputAxis|MoveRIght`
  (params (AxisValue :type "Float (single-precision)"))
  ;[1 1 1] Player Input
  (bind _return_direction_speed (`self.Movement` AxisValue (`self.HSpeed`)))
  (set `self.HSpeed` _return_direction_speed))

(event `PFire`
  ;[1 1 1] Player Primary Fire
  (`self.PrimaryFire` (`SceneComponent.K2_GetComponentToWorld` (`self.ProjectileSpawn`)) :!label _label))

(event `InputAction|PrimaryFire`
  (params (Key :type "Key Structure"))
  ;[1 1 1] Player Primary Fire
  (:`Pressed`
    (if (`self.MoveEnabled`)
      (`KismetSystemLibrary.K2_SetTimer` null "PFire" 0.2 true)
      (goto _label)))
  (:`Released`
    (`KismetSystemLibrary.K2_ClearTimer` null "PFire")))

(event `SFire`
  ;[1 1 1] Player Secondary Fire
  (`self.SecondaryFire` (`SceneComponent.K2_GetComponentToWorld` (`self.ProjectileSpawnL`)) :!label _label_2)
  (`self.SecondaryFire` (`SceneComponent.K2_GetComponentToWorld` (`self.ProjectileSpawnR`))))

(event `InputAction|SecondaryFire`
  (params (Key :type "Key Structure"))
  ;[1 1 1] Player Secondary Fire
  (:`Pressed`
    (if (`self.MoveEnabled`)
      (`KismetSystemLibrary.K2_SetTimer` null "SFire" 0.6 true)
      (goto _label_2)))
  (:`Released`
    (`KismetSystemLibrary.K2_ClearTimer` null "SFire")))

(event `self.ReceiveAnyDamage`
  (params (Damage :type "Float (single-precision)") (DamageType :type "DamageType Object Reference") (InstigatedBy :type "Controller Object Reference") (DamageCauser :type "Actor Object Reference"))
  (bind _returnvalue (`self.K2_GetActorLocation`))
  (bind _bp_gamemode (`self.BP_GameMode`))
  ;[1 1 1] Player Damage
  (set `self.Health` (`KismetMathLibrary.FClamp` (- (`self.Health`) Damage) 0.0 (`self.MaxHealth`)))
  (`/Game/Blueprints/BP_GameMode.PlayCameraShake` (`self.BP_GameMode`) "/Game/Blueprints/CameraShakes/BP_CameraShakeSmall.BP_CameraShakeSmall_C" (`self.K2_GetActorLocation`))
  (if (<= (`self.Health`) 0.0)
    (`GameplayStatics.SpawnEmitterAtLocation` "/Game/Assets/Particles/P_Pixel_Explosion.P_Pixel_Explosion" _returnvalue)
    (`GameplayStatics.PlaySoundAtLocation` "/Game/Assets/Audio/Blueprints_TextPop01.Blueprints_TextPop01" _returnvalue)
    (`/Game/Blueprints/BP_GameMode.PlayCameraShake` _bp_gamemode "/Game/Blueprints/CameraShakes/BP_CameraShake.BP_CameraShake_C" (`self.K2_GetActorLocation`))
    (`/Game/Blueprints/BP_GameMode.GameOver` _bp_gamemode)
    (`self.K2_DestroyActor`)))

(event `self.BoxCollider.OnComponentHit`
  (params (HitComponent :type "PrimitiveComponent Object Reference") (OtherActor :type "Actor Object Reference") (OtherComp :type "PrimitiveComponent Object Reference") (NormalImpulse :type "Vector Structure") (Hit :type "HitResult Structure (by ref)"))
  ;[1 1 1] Player Collision
  (set `self.HSpeed` (* (* (`KismetMathLibrary.FClamp` (`KismetMathLibrary.Abs` (`self.HSpeed`)) 0.0 1.5) -2.0) (.x Hit_Normal)))
  (set `self.VSpeed` (* (* (`KismetMathLibrary.FClamp` (`KismetMathLibrary.Abs` (`self.VSpeed`)) 0.0 1.5) 2.0) (.z Hit_Normal))))

(fn `Movement`
  (params (Direction :type "Float (double-precision)") (Speed :type "Float (double-precision)"))
  (returns (`Return Direction Speed` :type "Float (double-precision)"))
  (return (`KismetMathLibrary.FInterpTo` Speed (* (* (`self.MovementSpeed`) Direction) (`self.DeltaSeconds`)) (`self.DeltaSeconds`) 12.0)))

(fn `PrimaryFire`
  (params (SpawnTransform :type "Transform Structure"))
  (locals (ProjectileColor :type "LinearColor Structure" :default (struct :`G` 0.30317 :`B` 1.0 :`A` 1.0)))
  (bind _returnvalue (`|SpawnActorFromClass` "/Game/Blueprints/Bullets/BP_BulletPlayer_Primary.BP_BulletPlayer_Primary_C" SpawnTransform "AlwaysSpawn" "OverrideRootScale" null (`local.ProjectileColor`) self))
  (`self.K2_AttachToActor` _returnvalue (`self.BP_ParallaxCamera`) "None" "KeepWorld" "KeepRelative" "KeepRelative" true)
  (`GameplayStatics.PlaySoundAtLocation` "/Game/Assets/Audio/Cleaver_ImpactLayerSpark01.Cleaver_ImpactLayerSpark01" (`self.K2_GetActorLocation`)))

(fn `SecondaryFire`
  (params (SpawnTransform :type "Transform Structure"))
  (locals (`Projectile Color` :type "LinearColor Structure" :default (struct :`R` 0.434154 :`G` 1.0 :`B` 0.001518 :`A` 1.0)))
  (bind _returnvalue (`|SpawnActorFromClass` "/Game/Blueprints/Bullets/BP_BulletPlayer_Secondary.BP_BulletPlayer_Secondary_C" SpawnTransform "AlwaysSpawn" "OverrideRootScale" null (`local.Projectile Color`) self))
  (`self.K2_AttachToActor` _returnvalue (`self.BP_ParallaxCamera`) "None" "KeepWorld" "KeepRelative" "KeepRelative" true)
  (`GameplayStatics.PlaySoundAtLocation` "/Game/Assets/Audio/Cleaver_ImpactLayerSpark03.Cleaver_ImpactLayerSpark03" (`self.K2_GetActorLocation`)))

(fn `UserConstructionScript`
  (set `self.Health` (`self.MaxHealth`)))