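; Player actor for a shooter that moves in the X-Z plane and fires colored projectiles.
; On spawn a timeline lifts and spins it, then sets MoveEnabled, which gates only firing.
; Axis inputs ease speeds that Tick applies as swept per-frame offsets, adding vertical twice, while the mesh yaws with horizontal speed.
; Held fire inputs run looping timers: primary spawns from one point, secondary from left and right at a slower rate.
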(event `self.ReceiveBeginPlay`
  (bind _spawnlocation (`self.SpawnLocation`))
  ;[1 1 1] Player Spawn Animation
  (bind _asbp_game_mode (cast `/Game/Blueprints/BP_GameMode` (`GameplayStatics.GetGameMode`)))
  (set `self.BP_GameMode` _asbp_game_mode)
  (set `self.Yaw` (.yaw (`self.K2_GetActorRotation`)))
  (set `self.SpawnLocation` (`self.K2_GetActorLocation`))
  (bind (_direction _speed) (`Timeline|SpawnAnimation`)
    (:`Update`
      (`self.K2_SetActorLocation` (`KismetMathLibrary.VLerp` _spawnlocation (+ _spawnlocation (0.0 0.0 60.0)) _speed))
      (`SceneComponent.K2_SetRelativeRotation` (`self.PlayerMesh`) (`KismetMathLibrary.RLerp` (struct) (`KismetMathLibrary.MakeRotator` 0.0 0.0 (+ (`self.Yaw`) (`self.SpawnSpinCount`))) _speed) false false))
    (:`Finished`
      (set `self.MoveEnabled` true))))

(event `self.ReceiveTick`
  (params (DeltaSeconds :type "Float (single-precision)"))
  (bind _playermesh (`self.PlayerMesh`))
  ;[1 1 1] Player Movement
  (set `self.DeltaSeconds` DeltaSeconds)
  (`self.K2_SetActorLocation` (+ (`self.K2_GetActorLocation`) (`KismetMathLibrary.MakeVector` (`self.HSpeed`) 0.0 (`self.VSpeed`))) true)
  (`self.K2_SetActorLocation` (+ (`self.K2_GetActorLocation`) (`KismetMathLibrary.MakeVector` 0.0 0.0 (`self.VSpeed`))) true)
  (`SceneComponent.K2_SetRelativeRotation` _playermesh (`KismetMathLibrary.RInterpTo_Constant` (`SceneComponent.RelativeRotation` _playermesh) (`KismetMathLibrary.MakeRotator` 0.0 0.0 (+ (* (`self.HSpeed`) -8.0) (`self.Yaw`))) (`self.DeltaSeconds`) 80.0) false false))

(event `InputAxis|MoveUp`
  (params (AxisValue :type "Float (single-precision)"))
  ;[1 1 1] Player Input
  (bind _return_direction_speed (`self.Movement` AxisValue (`self.VSpeed`)))
  (set `self.VSpeed` _return_direction_speed))

(event `InputAxis|MoveRIght`
  (params (AxisValue :type "Float (single-precision)"))
  ;[1 1 1] Player Input
  (bind _return_direction_speed (`self.Movement` AxisValue (`self.HSpeed`)))
  (set `self.HSpeed` _return_direction_speed))

(event `PFire`
  ;[1 1 1] Player Primary Fire
  (`self.PrimaryFire` (`SceneComponent.K2_GetComponentToWorld` (`self.ProjectileSpawn`)) :!label _label))

(event `InputAction|PrimaryFire`
  (params (Key :type "Key Structure"))
  ;[1 1 1] Player Primary Fire
  (:`Pressed`
    (if (`self.MoveEnabled`)
      (`KismetSystemLibrary.K2_SetTimer` null "PFire" 0.2 true)
      (goto _label)))
  (:`Released`
    (`KismetSystemLibrary.K2_ClearTimer` null "PFire")))

(event `SFire`
  ;[1 1 1] Player Secondary Fire
  (`self.SecondaryFire` (`SceneComponent.K2_GetComponentToWorld` (`self.ProjectileSpawnL`)) :!label _label_2)
  (`self.SecondaryFire` (`SceneComponent.K2_GetComponentToWorld` (`self.ProjectileSpawnR`))))

(event `InputAction|SecondaryFire`
  (params (Key :type "Key Structure"))
  ;[1 1 1] Player Secondary Fire
  (:`Pressed`
    (if (`self.MoveEnabled`)
      (`KismetSystemLibrary.K2_SetTimer` null "SFire" 0.6 true)
      (goto _label_2)))
  (:`Released`
    (`KismetSystemLibrary.K2_ClearTimer` null "SFire")))

(fn `Movement`
  (params (Direction :type "Float (double-precision)") (Speed :type "Float (double-precision)"))
  (returns (`Return Direction Speed` :type "Float (double-precision)"))
  (return (`KismetMathLibrary.FInterpTo` Speed (* (`self.MovementSpeed`) Direction) (`self.DeltaSeconds`) 12.0)))

(fn `PrimaryFire`
  (params (SpawnTransform :type "Transform Structure"))
  (locals (ProjectileColor :type "LinearColor Structure" :default (struct :`R` 0.017018 :`G` 1.0 :`B` 0.555887)))
  (`|SpawnActorFromClass` "/Game/Blueprints/BP_ProjectilePlayerBase.BP_ProjectilePlayerBase_C" SpawnTransform "AlwaysSpawn" "OverrideRootScale" null (`local.ProjectileColor`) self))

(fn `SecondaryFire`
  (params (SpawnTransform :type "Transform Structure"))
  (locals (`Projectile Color` :type "LinearColor Structure" :default (struct :`R` 0.786429 :`B` 1.0)))
  (`|SpawnActorFromClass` "/Game/Blueprints/BP_ProjectilePlayerBase.BP_ProjectilePlayerBase_C" SpawnTransform "AlwaysSpawn" "OverrideRootScale" null (`local.Projectile Color`) self))

(fn `UserConstructionScript`)