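; Enemy squadron actor that holds one enemy of a configurable class and hands it to the game mode when triggered.
; On BeginPlay it spawns the enemy and attaches it to itself with relative transform rules.
; Any actor overlap prints the other actor's name, then calls AddEnemy on BP_GameMode with the enemy and a BulletML movement file path.
; The overlap is neither filtered nor limited to one trigger.
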(event `self.ReceiveBeginPlay`
  (bind _returnvalue (`|SpawnActorFromClass` (`self.BP_EnemyClass`) (`KismetMathLibrary.MakeTransform` (0.0 0.0 0.0)) "Undefined" "OverrideRootScale" null null))
  (bind _output_get (set `self.BP_EnemyActor` _returnvalue))
  (`self.K2_AttachToActor` _output_get self "None" "KeepRelative" "KeepRelative" "KeepRelative" true))

(event `self.ReceiveActorBeginOverlap`
  (params (OtherActor :type "Actor Object Reference"))
  (`KismetSystemLibrary.PrintString` (`KismetSystemLibrary.GetDisplayName` OtherActor))
  (bind _asbp_game_mode (cast `/Game/Blueprints/BP_GameMode` (`GameplayStatics.GetGameMode`)))
  (`GameManager.AddEnemy` _asbp_game_mode (`self.BP_EnemyActor`) (`.FilePath` (break `FilePath` (`self.MoveBulletML`)))))

(fn `UserConstructionScript`)