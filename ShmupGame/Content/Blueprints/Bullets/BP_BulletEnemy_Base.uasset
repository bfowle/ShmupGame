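; Base enemy projectile that damages the player on hit.
; The construction script creates a dynamic material on the Projectile component and applies its scale; BeginPlay then tints that material with the projectile color.
; A component hit applies damage only to BP_Player and destroys the bullet whatever it struck.
; Tick is empty despite its off-screen removal label, and some cast logic is disconnected.
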(event `self.ReceiveBeginPlay`
  ;[1 1 1] Setup
  (`MaterialInstanceDynamic.SetVectorParameterValue` (`self.ProjectileMaterial`) "Color" (`self.ProjectileColor`)))

(event `self.ReceiveTick`
  (params (DeltaSeconds :type "Float (single-precision)"))
  ;[1 1 1] Remove when actor leaves screen viewport
)

(event `self.Projectile.OnComponentHit`
  (params (HitComponent :type "PrimitiveComponent Object Reference") (OtherActor :type "Actor Object Reference") (OtherComp :type "PrimitiveComponent Object Reference") (NormalImpulse :type "Vector Structure") (Hit :type "HitResult Structure (by ref)"))
  ;[1 1 1] Remove when hit, damages another actor
  (bind _asbp_player (cast `/Game/Blueprints/Player/BP_Player` OtherActor)
    (:`then`
      (`GameplayStatics.ApplyDamage` _asbp_player (`self.Damage`)))
    (:`CastFailed`
      _))
  (`self.K2_DestroyActor`))

(fn `UserConstructionScript`
  (bind _returnvalue (`PrimitiveComponent.CreateDynamicMaterialInstance` (`self.Projectile`) 0 null))
  (set `self.ProjectileMaterial` _returnvalue)
  (`SceneComponent.SetWorldScale3D` (`self.Projectile`) (`self.Scale`)))