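; Base Blueprint for player projectiles, with configurable color, scale and speed.
; The construction script creates a dynamic material instance on the Projectile component, applies the world scale, and sets the movement component's initial and max speed from Speed.
; On BeginPlay it writes the projectile color into the material's Color parameter.
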(event `self.ReceiveBeginPlay`
  (`MaterialInstanceDynamic.SetVectorParameterValue` (`self.ProjectileMaterial`) "Color" (`self.ProjectileColor`)))

(fn `UserConstructionScript`
  (bind _projectilemovement (`self.ProjectileMovement`))
  (bind _returnvalue (`PrimitiveComponent.CreateDynamicMaterialInstance` (`self.Projectile`) 0 null))
  (set `self.ProjectileMaterial` _returnvalue)
  (`SceneComponent.SetWorldScale3D` (`self.Projectile`) (`self.Scale`))
  (bind _output_get (set `ProjectileMovementComponent.MaxSpeed` (`self.Speed`) _projectilemovement))
  (set `ProjectileMovementComponent.InitialSpeed` _output_get _projectilemovement))