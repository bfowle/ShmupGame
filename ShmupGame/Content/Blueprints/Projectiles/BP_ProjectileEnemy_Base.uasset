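; Base enemy projectile that damages the player on hit and destroys itself on any hit.
; The construction script scales the projectile mesh and creates a dynamic material instance, which is tinted with the projectile color at BeginPlay.
; On a component hit it applies damage only to BP_Player, then destroys itself and removes itself from the GameManager game mode's bullet tracking.
; A world-static collision check is present but disconnected.
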(event `self.ReceiveBeginPlay`
  (`MaterialInstanceDynamic.SetVectorParameterValue` (`self.ProjectileMaterial`) "Color" (`self.ProjectileColor`)))

(event `self.Projectile.OnComponentHit`
  (params (HitComponent :type "PrimitiveComponent Object Reference") (OtherActor :type "Actor Object Reference") (OtherComp :type "PrimitiveComponent Object Reference") (NormalImpulse :type "Vector Structure") (Hit :type "HitResult Structure (by ref)"))
  (bind _asbp_player (cast `/Game/Blueprints/Player/BP_Player` OtherActor)
    (:`then`
      (`GameplayStatics.ApplyDamage` _asbp_player (`self.Damage`)))
    (:`CastFailed`
      _))
  (`self.K2_DestroyActor`)
  (bind _asgame_manager (cast `GameManager` (`GameplayStatics.GetGameMode`)))
  (`GameManager.RemoveBullet` _asgame_manager self))

(fn `UserConstructionScript`
  (bind _returnvalue (`PrimitiveComponent.CreateDynamicMaterialInstance` (`self.Projectile`) 0 null))
  (set `self.ProjectileMaterial` _returnvalue)
  (`SceneComponent.SetWorldScale3D` (`self.Projectile`) (`self.Scale`)))