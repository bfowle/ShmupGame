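; Asteroid enemy Blueprint that moves by projectile movement and awards score when destroyed.
; On BeginPlay it caches BP_GameMode, then randomizes its speed and per-axis mesh scale within min/max ranges, giving non-uniform shapes.
; The construction script runs the parent's and applies the current Scale value to the mesh.
; EnemyKilled passes its score value to the game mode, requests a camera shake at its location, plays a pop sound and destroys the actor.
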(event `self.ReceiveBeginPlay`
  (bind _projectilemovement (`self.ProjectileMovement`))
  (bind _returnvalue (`KismetMathLibrary.RandomFloatInRange` (`self.MinScale`) (`self.MaxScale`)))
  ;[1 1 1] Asteroid Setup References and Variables
  (bind _asbp_game_mode (cast `/Game/Blueprints/BP_GameMode` (`GameplayStatics.GetGameMode`)))
  (set `self.BP_GameMode` _asbp_game_mode)
  (bind _output_get (set `self.MovementSpeed` (`KismetMathLibrary.RandomFloatInRange` (`self.MinSpeed`) (`self.MaxSpeed`))))
  (bind _output_get_2 (set `ProjectileMovementComponent.MaxSpeed` _output_get _projectilemovement))
  (set `ProjectileMovementComponent.InitialSpeed` _output_get_2 _projectilemovement)
  (bind _output_get_3 (set `self.Scale` (`KismetMathLibrary.MakeVector` _returnvalue _returnvalue _returnvalue)))
  (`SceneComponent.SetWorldScale3D` (`self.StaticMesh`) _output_get_3))

(event `self.EnemyKilled`
  (params (Location :type "Vector Structure"))
  (bind _returnvalue (`self.K2_GetActorLocation`))
  (bind _bp_gamemode (`self.BP_GameMode`))
  ;[1 1 1] Asteroid Destroyed
  (`/Game/Blueprints/BP_GameMode.SetScore` _bp_gamemode (`self.EnemyScoreValue`))
  (`/Game/Blueprints/BP_GameMode.PlayCameraShake` _bp_gamemode "/Script/Engine.CameraShake" _returnvalue)
  (`GameplayStatics.PlaySoundAtLocation` "/Game/Assets/Audio/Blueprints_TextPop01.Blueprints_TextPop01" _returnvalue)
  (`self.K2_DestroyActor`))

(fn `UserConstructionScript`
  (`parent.UserConstructionScript`)
  (`SceneComponent.SetWorldScale3D` (`self.StaticMesh`) (`self.Scale`)))