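; Base enemy for what appears to be a side-to-side shooter, registering with BP_GameMode and randomizing its speed and direction on spawn.
; Non-projectile hits flip its direction, while player contact damages the player and kills it, as does depleted health.
; EnemyKilled updates score, plays explosion, shake and sound, then destroys it.
; Horizontal movement, the drop-in timeline and the proximity-based FireNode shot exist but are unwired.
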(event `self.ReceiveBeginPlay`
  ;[1 1 1] Enemy Setup References and Variables
  (bind _asbp_game_mode (cast `/Game/Blueprints/BP_GameMode` (`GameplayStatics.GetGameMode`)))
  (bind _output_get (set `self.BP_GameMode` _asbp_game_mode))
  (`/Game/Blueprints/BP_GameMode.UpdateEnemyCount` _output_get 1)
  (set `self.MoveDirection` (`KismetMathLibrary.RandomBool`))
  (set `self.MovementSpeed` (`KismetMathLibrary.RandomFloatInRange` (`self.MinSpeed`) (`self.MaxSpeed`)))
  (set `self.SpawnLocation` (`self.K2_GetActorLocation`)))

(event `self.ReceiveTick`
  (params (DeltaSeconds :type "Float (single-precision)"))
  ;[1 1 1] Enemy Movement
)

(event `self.ReceiveHit`
  (params (MyComp :type "PrimitiveComponent Object Reference") (Other :type "Actor Object Reference") (OtherComp :type "PrimitiveComponent Object Reference") (bSelfMoved :type Boolean) (HitLocation :type "Vector Structure") (HitNormal :type "Vector Structure") (NormalImpulse :type "Vector Structure") (Hit :type "HitResult Structure (by ref)"))
  ;[1 1 1] Enemy Damage
  (cast `/Game/Blueprints/Projectiles/BP_ProjectilePlayer_Base` Other
    (:`CastFailed`
      (set `self.MoveDirection` (not (`self.MoveDirection`)))
      (bind _asbp_player (cast `/Game/Blueprints/Player/BP_Player` Other))
      (`GameplayStatics.ApplyDamage` _asbp_player 50.0)
      (`self.EnemyKilled` (`self.K2_GetActorLocation`) :!label _label))))

(event `self.ReceiveAnyDamage`
  (params (Damage :type "Float (single-precision)") (DamageType :type "DamageType Object Reference") (InstigatedBy :type "Controller Object Reference") (DamageCauser :type "Actor Object Reference"))
  ;[1 1 1] Enemy Damage
  (set `self.Health` (`KismetMathLibrary.FClamp` (- (`self.Health`) Damage) 0.0 (`self.MaxHealth`)))
  (if (<= (`self.Health`) 0.0)
    (goto _label)))

(fn `EnemyKilled`
  (params (Location :type "Vector Structure"))
  (bind _returnvalue (`self.K2_GetActorLocation`))
  (bind _bp_gamemode (`self.BP_GameMode`))
  (`GameplayStatics.SpawnEmitterAtLocation` "/Game/Assets/Particles/P_Pixel_Explosion_Player.P_Pixel_Explosion_Player" Location)
  (`/Game/Blueprints/BP_GameMode.EnemyKilled` _bp_gamemode)
  (`/Game/Blueprints/BP_GameMode.SetScore` _bp_gamemode (`self.EnemyScoreValue`))
  (`/Game/Blueprints/BP_GameMode.PlayCameraShake` _bp_gamemode "/Game/Blueprints/CameraShakes/BP_CameraShake.BP_CameraShake_C" _returnvalue)
  (`GameplayStatics.PlaySoundAtLocation` "/Game/Assets/Audio/Blueprints_TextPop01.Blueprints_TextPop01" _returnvalue)
  (`self.K2_DestroyActor`))

(fn `UserConstructionScript`
  (`AddComponent|NODE_AddEnemyComponent-0`))