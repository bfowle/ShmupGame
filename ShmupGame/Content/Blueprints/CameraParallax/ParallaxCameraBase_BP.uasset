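; Side-scrolling camera actor that optionally follows a character and scrolls background actors for a parallax effect.
; When following, Tick clamps camera X to set bounds and adds the character's vertical delta, jumps included.
; ParallaxLayers shifts each background along X by the camera's movement since the last update, scaled by a per-layer factor.
; The construction script positions the camera, converts enum presets into factors and optionally configures a farplane mesh.
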(event `self.ReceiveTick`
  (params (DeltaSeconds :type "Float (single-precision)"))
  (bind _cameraclamps (`self.CameraClamps`))
  (bind (__characterfollowlocation_x __characterfollowlocation_y __characterfollowlocation_z) (`KismetMathLibrary.BreakVector` (`self._characterFollowLocation`)))
  (bind (_returnvalue_x _returnvalue_y _returnvalue_z) (`KismetMathLibrary.BreakVector` (`self.K2_GetActorLocation` (`self.CharacterToFollow`))))
  (bind _returnvalue_x_2 (`KismetMathLibrary.BreakVector` (`self.K2_GetActorLocation` (`self.CharacterToFollow`))))
  (bind (_returnvalue_x_3 _returnvalue_y_2 _returnvalue_z_2) (`KismetMathLibrary.BreakVector` (`self.K2_GetActorLocation` self)))
  (if (`self.FollowCharacter`)
    ;[0 0.2919 1] Camera Movement
    ;;[1 1 1] Check to see if the player has moved
    (if (!= (`self.K2_GetActorLocation` (`self.CharacterToFollow`)) (`self._characterFollowLocation`))
      ;;[1 1 1] Get character delta
      (bind _output_get (set `self._characterZDelta` (- _returnvalue_z __characterfollowlocation_z)))
      ;;[1 1 1] Add delta Z. If the camera should not follow the character's jump, reroute around this.
      (`self.K2_AddActorWorldOffset` self (`KismetMathLibrary.MakeVector` 0.0 0.0 _output_get) false false)
      ;;[1 1 1] Move X and clamp
      (`self.K2_SetActorLocation` self (`KismetMathLibrary.MakeVector` (`KismetMathLibrary.FClamp` _returnvalue_x_2 (`|GetArrayItem` _cameraclamps) (`|GetArrayItem` _cameraclamps 1)) _returnvalue_y_2 _returnvalue_z_2) false false)
      ;;[1 1 1] Reset character location
      (bind _output_get_2 (set `self._characterFollowLocation` (`self.K2_GetActorLocation` (`self.CharacterToFollow`))))
      (`KismetSystemLibrary.PrintString` (`KismetStringLibrary.Conv_VectorToString` _output_get_2))
      (`self.ParallaxLayers`))
    (else
      (`self.ParallaxLayers`))))

(event `ParallaxLayers`
  (bind __lastposition_x (`KismetMathLibrary.BreakVector` (`self._lastPosition`)))
  (bind _returnvalue_x (`KismetMathLibrary.BreakVector` (`self.K2_GetActorLocation` self)))
  ;[1 1 1] Parallax Movement
  ;;[1 1 1] Calculate camera position delta change
  (set `self._parallaxDelta` (- __lastposition_x _returnvalue_x))
  ;;[1 1 1] Loop through "Background" objects
  (for _index (range (`KismetArrayLibrary.Array_Length` (`self.Backgrounds`)))
    (bind _returnvalue_x_2 (`KismetMathLibrary.BreakVector` (`self.K2_GetActorLocation` (`|GetArrayItem` (`self.Backgrounds`) _index))))
    ;;[1 1 1] Set parallax layer locations
    (bind _output_get (set `self._backgroundTargetPosition` (- _returnvalue_x_2 (* (`|GetArrayItem` (`self.ParallaxFactor`) _index) (`self._parallaxDelta`)))))
    (bind _output (`|GetArrayItem` (`self.Backgrounds`) _index))
    (bind (_returnvalue_x_3 _returnvalue_y _returnvalue_z) (`KismetMathLibrary.BreakVector` (`self.K2_GetActorLocation` _output)))
    (`self.K2_SetActorLocation` _output (`KismetMathLibrary.MakeVector` _output_get _returnvalue_y _returnvalue_z) false false))
  ;;[1 1 1] Store last position
  (set `self._lastPosition` (`self.K2_GetActorLocation` self)))

(fn `UserConstructionScript`
  ;[1 1 1] Initial Camera Settings
  (bind _output_get (set `self._characterFollowLocation` (`self.K2_GetActorLocation` (`self.CharacterToFollow`))))
  (if (`self.FollowCharacter`)
    (`self.K2_SetActorLocation` self _output_get false false)
    (`self.K2_AddActorLocalOffset` self (`self.CameraOffset`) false false))
  ;[1 1 1] Get the initial camera position
  (set `self._lastPosition` (`self.K2_GetActorLocation` self))
  (`|ExecutionSequence`
    (:`then_0`
      ;[0.2549 1 0.4353] Set parallax preset values
      (for _index (range (`KismetArrayLibrary.Array_Length` (`self.PresetEnum`)))
        (if (`|EnumEquality` (`|GetArrayItem` (`self.PresetEnum`) _index) "NewEnumerator1")
          (`KismetArrayLibrary.Array_Set` (`self.ParallaxFactor`) _index -2.0 true)
          (elif (`|EnumEquality` (`|GetArrayItem` (`self.PresetEnum`) _index) "NewEnumerator0")
            (`KismetArrayLibrary.Array_Set` (`self.ParallaxFactor`) _index 0.2 true)
            (elif (`|EnumEquality` (`|GetArrayItem` (`self.PresetEnum`) _index) "NewEnumerator2")
              (`KismetArrayLibrary.Array_Set` (`self.ParallaxFactor`) _index 0.5 true)
              (elif (`|EnumEquality` (`|GetArrayItem` (`self.PresetEnum`) _index) "NewEnumerator3")
                (`KismetArrayLibrary.Array_Set` (`self.ParallaxFactor`) _index 0.75 true)))))))
    (:`then_1`
      ;[1 1 1] Farplane settings
      (if (`self.Use Farplane`)
        (`StaticMeshComponent.SetStaticMesh` (`self.FarplaneMesh`))
        (`SceneComponent.K2_SetRelativeLocationAndRotation` (`self.FarplaneLocation`) (`self.FarplaneRotation`))
        (`SceneComponent.SetRelativeScale3D` (`self.FarplaneScale`))
        (`PrimitiveComponent.SetMaterial` 0 (`self.FarplaneMaterial`))))))