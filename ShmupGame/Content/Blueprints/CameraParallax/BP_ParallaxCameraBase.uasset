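; Base parallax camera actor that scrolls an array of background actors to fake depth as the camera moves along X.
; Each Tick scales the camera's X movement by a per-layer factor and shifts the matching background, preserving Y and Z.
; The construction script optionally snaps the camera to a character plus offset, converts per-layer enum presets into factors, and optionally configures a farplane mesh.
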(event `self.ReceiveTick`
  (params (DeltaSeconds :type "Float (single-precision)"))
  (bind __lastposition_x (`KismetMathLibrary.BreakVector` (`self._lastPosition`)))
  (bind _returnvalue_x (`KismetMathLibrary.BreakVector` (`self.K2_GetActorLocation` self)))
  ;[1 1 1] Parallax Movement
  ;;[1 1 1] Calculate camera position delta change
  (set `self._parallaxDelta` (- __lastposition_x _returnvalue_x))
  ;;[1 1 1] Loop through "Background" objects
  (for _index (range (`KismetArrayLibrary.Array_Length` (`self.Backgrounds`)))
    (bind _returnvalue_x_2 (`KismetMathLibrary.BreakVector` (`self.K2_GetActorLocation` (`|GetArrayItem` (`self.Backgrounds`) _index))))
    ;;[1 1 1] Set parallax layer locations
    (bind _output_get (set `self._backgroundTargetPosition` (- _returnvalue_x_2 (* (`|GetArrayItem` (`self.ParallaxFactor`) _index) (`self._parallaxDelta`)))))
    (bind _output (`|GetArrayItem` (`self.Backgrounds`) _index))
    (bind (_returnvalue_x_3 _returnvalue_y _returnvalue_z) (`KismetMathLibrary.BreakVector` (`self.K2_GetActorLocation` _output)))
    (`self.K2_SetActorLocation` _output (`KismetMathLibrary.MakeVector` _output_get _returnvalue_y _returnvalue_z) false false))
  ;;[1 1 1] Store last position
  (set `self._lastPosition` (`self.K2_GetActorLocation` self)))

(fn `UserConstructionScript`
  ;[1 1 1] Initial Camera Settings
  (bind _output_get (set `self._characterFollowLocation` (`self.K2_GetActorLocation` (`self.CharacterToFollow`))))
  (if (`self.FollowCharacter`)
    (`self.K2_SetActorLocation` self _output_get false false)
    (`self.K2_AddActorLocalOffset` self (`self.CameraOffset`) false false))
  ;[1 1 1] Get the initial camera position
  (set `self._lastPosition` (`self.K2_GetActorLocation` self))
  (`|ExecutionSequence`
    (:`then_0`
      ;[0.2549 1 0.4353] Set parallax preset values
      (for _index (range (`KismetArrayLibrary.Array_Length` (`self.PresetEnum`)))
        (if (`|EnumEquality` (`|GetArrayItem` (`self.PresetEnum`) _index) "NewEnumerator1")
          (`KismetArrayLibrary.Array_Set` (`self.ParallaxFactor`) _index -2.0 true)
          (elif (`|EnumEquality` (`|GetArrayItem` (`self.PresetEnum`) _index) "NewEnumerator0")
            (`KismetArrayLibrary.Array_Set` (`self.ParallaxFactor`) _index 0.2 true)
            (elif (`|EnumEquality` (`|GetArrayItem` (`self.PresetEnum`) _index) "NewEnumerator2")
              (`KismetArrayLibrary.Array_Set` (`self.ParallaxFactor`) _index 0.5 true)
              (elif (`|EnumEquality` (`|GetArrayItem` (`self.PresetEnum`) _index) "NewEnumerator3")
                (`KismetArrayLibrary.Array_Set` (`self.ParallaxFactor`) _index 0.75 true)))))))
    (:`then_1`
      ;[1 1 1] Farplane settings
      (if (`self.Use Farplane`)
        (`StaticMeshComponent.SetStaticMesh` (`self.FarplaneMesh`))
        (`SceneComponent.K2_SetRelativeLocationAndRotation` (`self.FarplaneLocation`) (`self.FarplaneRotation`))
        (`SceneComponent.SetRelativeScale3D` (`self.FarplaneScale`))
        (`PrimitiveComponent.SetMaterial` 0 (`self.FarplaneMaterial`))))))