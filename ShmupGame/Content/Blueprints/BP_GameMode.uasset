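; BP_GameMode is a game mode that tracks score and enemy counts, creates the HUD on BeginPlay and handles game over.
; SetScore adds to the score and EnemyKilled updates both kill and remaining counts, while PlayCameraShake triggers a world shake at an epicenter.
; GameOver shows its widget with a cursor and UI-only input.
; LoadScore and SaveScore are empty stubs, and the TopScore comparison is unwired.
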(event `self.ReceiveBeginPlay`
  ;[1 1 1] Game Begin
  (`WidgetBlueprintLibrary.SetInputMode_GameOnly` (`GameplayStatics.GetPlayerController` 0))
  (`self.LoadScore`)
  (`self.SetScore` 0)
  (bind _returnvalue (`|CreateWidget` "/Game/Blueprints/Widgets/BPW_HUD.BPW_HUD_C"))
  (bind _output_get (set `self.BPW_HUD` _returnvalue))
  (`UserWidget.AddToViewport` _output_get 0))

(event `self.ReceiveEndPlay`
  (params (EndPlayReason :type "EEndPlayReason Enum" :default "Destroyed"))
  ;[1 1 1] Game End
  (`self.SaveScore`))

(fn `EnemyKilled`
  (`/Engine/EditorBlueprintResources/StandardMacros.IncrementInt` (`self.EnemiesKilled`)
    (:`  `
      (`self.UpdateEnemyCount` -1))))

(fn `GameOver`
  (bind _returnvalue (`GameplayStatics.GetPlayerController` 0))
  (bind _returnvalue_2 (`|CreateWidget` "/Game/Blueprints/Widgets/BPW_GameOver.BPW_GameOver_C"))
  (`UserWidget.AddToViewport` _returnvalue_2 0)
  (set `PlayerController.bShowMouseCursor` true _returnvalue)
  (`WidgetBlueprintLibrary.SetInputMode_UIOnlyEx` _returnvalue _returnvalue_2))

(fn `LoadScore`)

(fn `PlayCameraShake`
  (params (Shake :type "CameraShake Class Reference") (Epicenter :type "Vector Structure"))
  (`GameplayStatics.PlayWorldCameraShake` Shake Epicenter 0.0 1000.0))

(fn `SaveScore`)

(fn `SetScore`
  (params (Value :type Integer))
  (bind _output_get (set `self.Score` (+ (`self.Score`) Value))))

(fn `UpdateEnemyCount`
  (params (Value :type Integer))
  (set `self.EnemyCount` (+ (`self.EnemyCount`) Value)))

(fn `UserConstructionScript`)